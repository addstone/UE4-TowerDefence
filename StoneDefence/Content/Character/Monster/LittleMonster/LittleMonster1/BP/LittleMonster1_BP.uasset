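; LittleMonster1_BP is the Blueprint for a little monster character, assembling its body components on the skeletal mesh.
; Its construction script runs the parent script, then attaches head, fire, left and right, joint and tail components to named sockets on Mesh.
; Each attachment snaps location to its socket while keeping world rotation and scale.
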(fn ConstructionScript
  (bind _mesh (Variables|Character|GetMesh))
  (|CallParentFunction)
  (Transformation|AttachComponentToComponent (Variables|Default|GetHead) _mesh "Head" "SnapToTarget" "KeepWorld" "KeepWorld" true)
  (Transformation|AttachComponentToComponent (Variables|Default|GetFire) _mesh "Fire" "SnapToTarget" "KeepWorld" "KeepWorld" true)
  (Transformation|AttachComponentToComponent (Variables|Default|GetL) _mesh "L" "SnapToTarget" "KeepWorld" "KeepWorld" true)
  (Transformation|AttachComponentToComponent (Variables|Default|GetR) _mesh "R" "SnapToTarget" "KeepWorld" "KeepWorld" true)
  (Transformation|AttachComponentToComponent (Variables|Default|GetL_Joint) _mesh "L_Jonit" "SnapToTarget" "KeepWorld" "KeepWorld" true)
  (Transformation|AttachComponentToComponent (Variables|Default|GetR_Joint) _mesh "R_Joint" "SnapToTarget" "KeepWorld" "KeepWorld" true)
  (Transformation|AttachComponentToComponent (Variables|Default|GetTail) _mesh "Tail" "SnapToTarget" "KeepWorld" "KeepWorld" true))